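; BP_DestructibleFiller is a destructible prop actor that supports a temporary custom-depth highlight, apparently for an outline effect.
; The construction script applies the DestructMesh variable to its DestructibleComponent.
; Destruct raises the Outline flag for a brief window without breaking the mesh itself.
; Interface event ChangeDepth enables custom depth with a stencil value only while that flag is set, and DisableDepth turns it off.
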(event EventDestruct
  (params (Mode :type PistolMode%20Enum :default "NewEnumerator0"))
  (Variables|Default|SetOutline true)
  (Utilities|FlowControl|Delay 1.0)
  (Variables|Default|SetOutline false))

(event EventChangeDepth
  (bind _destructiblecomponent (Variables|Default|GetDestructibleComponent))
  ;[1 1 1] Eventos Interface
  (if (Variables|Default|GetOutline)
    (Rendering|SetRenderCustomDepth _destructiblecomponent true)
    (Rendering|SetCustomDepthStencilValue _destructiblecomponent 2)))

(event EventDisableDepth
  ;[1 1 1] Eventos Interface
  (Rendering|SetRenderCustomDepth (Variables|Default|GetDestructibleComponent) false))

(fn ConstructionScript
  (Class|DestructibleComponent|SetDestructibleMesh (Variables|Default|GetDestructibleComponent) (Variables|Default|GetDestructMesh)))