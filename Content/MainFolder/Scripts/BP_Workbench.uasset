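; Workbench where a player carrying a toolbox holds Interact to unlock a laser mode: Construction, Destruction or Gravity, per the character's UpgradeMode.
; Box overlap outlines the mesh and enables input with a hold widget, or shows a toolbox widget when an armed player lacks one.
; A retriggerable delay completes the upgrade, consuming the toolbox and showing a tutorial.
; A parallel timer, polled by a zero-delay loop, drives the hold progress.
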(event OnComponentEndOverlap(Box)
  (params (OverlappedComponent :type Primitive%20Component%20Object%20Reference) (OtherActor :type Actor%20Object%20Reference) (OtherComp :type Primitive%20Component%20Object%20Reference) (OtherBodyIndex :type Integer))
  (bind _toolboxwidget (Variables|Default|GetToolboxWidget))
  ;[1 1 1] SetCustomDepth
  (Utilities|Casting|CastToBP_Character OtherActor)
  (Variables|Default|SetIsHeld? false)
  (Rendering|SetRenderCustomDepth (Variables|Default|GetStaticMesh) false)
  ;[1 1 1] Enable Input Character and add Widget to Viewport
  (Utilities|IsValid (Variables|Default|GetHoldWidget)
    (:Is%20Valid
      (Input|DisableInput (Game|GetPlayerController 0))
      (Widget|RemovefromParent (Variables|Default|GetHoldWidget))
      (UserInterface|Animation|PlayAnimation _toolboxwidget (Variables|/Game/MainFolder/UI/ToolboxUI/ToolboxWidget.ToolboxWidget_C|GetOut _toolboxwidget) 0.0 1 "Forward" 1.0 false)
      (Utilities|FlowControl|Delay 0.25)
      (Widget|RemovefromParent _toolboxwidget)
      ;[1 1 1] Player Has ToolBox?
      (Utilities|FlowControl|Gate true) ; enters at Close
    )))

(event OnComponentBeginOverlap(Box)
  (params (OverlappedComponent :type Primitive%20Component%20Object%20Reference) (OtherActor :type Actor%20Object%20Reference) (OtherComp :type Primitive%20Component%20Object%20Reference) (OtherBodyIndex :type Integer) (bFromSweep :type Boolean) (SweepResult :type Hit%20Result%20Structure%20%28by%20ref%29))
  (bind _holdwidget (Variables|Default|GetHoldWidget))
  (bind _staticmesh (Variables|Default|GetStaticMesh))
  ;[1 1 1] SetCustomDepth
  (bind _asbp_character (Utilities|Casting|CastToBP_Character OtherActor))
  (bind _output_get (Variables|Default|SetAs%20BP%20Character _asbp_character))
  (if (Variables|/Game/MainFolder/Scripts/BP_Character.BP_Character_C|GetHasToolBox (Variables|Default|GetAs%20BP%20Character))
    (Rendering|SetRenderCustomDepth _staticmesh true)
    ;[1 1 1] Enable Input Character and add Widget to Viewport
    (Rendering|SetCustomDepthStencilValue _staticmesh 4)
    (Utilities|IsValid (Variables|Default|GetHoldWidget)
      (:Is%20Valid
        (Input|EnableInput (Game|GetPlayerController 0))
        (UserInterface|Viewport|AddtoViewport _holdwidget 0)
        (Variables|/Game/MainFolder/UI/Hold_Widget.Hold_Widget_C|SetMaxTimeHeld _holdwidget (Variables|Default|GetMax%20Time%20Held))
        ;[1 1 1] Player Has ToolBox?
        (Utilities|FlowControl|Gate true) ; enters at Open
      ))
    (elif (Variables|/Game/MainFolder/Scripts/BP_Character.BP_Character_C|GetCanShoot _output_get)
      (UserInterface|Viewport|AddtoViewport (Variables|Default|GetToolboxWidget) 0))))

(event Custom|Timer
  ;[1 1 1] Timer
  (bind _returnvalue (Utilities|Time|SetTimerbyEvent (delegate Custom|Timer) (Variables|Default|GetMax%20Time%20Held))))

(event Custom|Stop%20Timer
  ;[1 1 1] Timer
  (Utilities|Time|PauseTimerbyHandle (stale Custom|Timer _returnvalue)))

(event Custom|UpdateTimer
  (bind _holdwidget (Variables|Default|GetHoldWidget))
  ;[1 1 1] Timer
  (if (Variables|Default|GetIsHeld?)
    (Variables|/Game/MainFolder/UI/Hold_Widget.Hold_Widget_C|SetTimeHeld _holdwidget (Class|KismetSystemLibrary|GetTimerElapsedTimeHandle (stale Custom|Timer _returnvalue)))
    (Utilities|FlowControl|Delay 0.0)
    (CallFunction|UpdateTimer)
    (else
      (CallFunction|StopTimer)
      (Variables|/Game/MainFolder/UI/Hold_Widget.Hold_Widget_C|SetTimeHeld _holdwidget 0.0))))

(event EventBeginPlay
  (Utilities|FlowControl|Sequence
    (:then_0
      (bind _returnvalue (UserInterface|CreateWidget "/Game/MainFolder/UI/Hold_Widget.Hold_Widget_C" (Game|GetPlayerController 0)))
      (Variables|Default|SetHoldWidget _returnvalue))
    (:then_1
      (bind _returnvalue_2 (UserInterface|CreateWidget "/Game/MainFolder/UI/ToolboxUI/ToolboxWidget.ToolboxWidget_C"))
      (Variables|Default|SetToolboxWidget _returnvalue_2))))

(event Input|ActionEvents|InputActionInteract
  (params (Key :type Key%20Structure :default "None"))
  (:Pressed
    (Variables|Default|SetIsHeld? true)
    ;[1 1 1] Player Has ToolBox?
    (Utilities|FlowControl|Gate true :!label _label
      (:Exit
        (Audio|PlaySound2D "/Game/MainFolder/Assets/Sounds/UpgradeWeapon_Cue.UpgradeWeapon_Cue" 1.0 1.0 0.0 0 0)
        ;[1 1 1] Init Held Widget
        (Utilities|FlowControl|Sequence
          (:then_0
            (Utilities|FlowControl|RetriggerableDelay (Variables|Default|GetMax%20Time%20Held))
            (if (Variables|Default|GetIsHeld?)
              (Rendering|SetRenderCustomDepth (Variables|Default|GetStaticMesh) false)
              (Rendering|SetVisibility (Variables|/Game/MainFolder/Scripts/BP_Character.BP_Character_C|GetSparks_P (Variables|Default|GetAs%20BP%20Character)) false false)
              (CallFunction|UpgradeLaserBehaviopur)
              (bind _returnvalue (UserInterface|CreateWidget "/Game/UI/TextBeforePickUP/TutorialWidget1.TutorialWidget1_C" (Game|GetPlayerController 0)))
              (bind _output_get (Variables|Default|SetTutorialWidgets _returnvalue))
              (Variables|/Game/UI/TextBeforePickUP/TutorialWidget1.TutorialWidget1_C|SetInputText _output_get (Utilities|String|Append (Variables|Default|GetTutorialString) (Variables|Default|GetStringMode) (Variables|Default|GetChangeModeTutorial)))
              (UserInterface|Viewport|AddtoViewport (Variables|Default|GetTutorialWidgets) 0)))
          (:then_1
            (CallFunction|Timer)
            (CallFunction|UpdateTimer))))))
  (:Released
    (Variables|Default|SetIsHeld? false)
    (goto _label)))

(fn ConstructionScript)

(fn UpgradeLaserBehaviopur
  (bind _as_bp_character (Variables|Default|GetAs%20BP%20Character))
  (bind _as_bp_character_2 (Variables|Default|GetAs%20BP%20Character))
  (switch Utilities|FlowControl|Switch|SwitchonUpgradeMode (Variables|/Game/MainFolder/Scripts/BP_Character.BP_Character_C|GetUpgradeMode (Variables|Default|GetAs%20BP%20Character))
    (:NewEnumerator0
      (Variables|/Game/MainFolder/Scripts/BP_Character.BP_Character_C|SetConstructionAvailable _as_bp_character true)
      (bind _output_get (Variables|/Game/MainFolder/Scripts/BP_Character.BP_Character_C|SetPistolMode _as_bp_character_2 "NewEnumerator1"))
      (Default|ChangetoConstruction _as_bp_character_2)
      (Variables|Default|SetStringMode (Utilities|String|EnumtoString _output_get)))
    (:NewEnumerator1
      (Variables|/Game/MainFolder/Scripts/BP_Character.BP_Character_C|SetDestructionAvailable _as_bp_character true)
      (bind _output_get_2 (Variables|/Game/MainFolder/Scripts/BP_Character.BP_Character_C|SetPistolMode _as_bp_character_2 "NewEnumerator2"))
      (Default|ChangetoDestruction _as_bp_character_2)
      (Variables|Default|SetStringMode (Utilities|String|EnumtoString _output_get_2)))
    (:NewEnumerator2
      (Variables|/Game/MainFolder/Scripts/BP_Character.BP_Character_C|SetGravityAvailable _as_bp_character true)
      (Default|ChangetoGravity _as_bp_character_2)
      (Variables|Default|SetStringMode "")))
  (Development|PrintString "Upgrade Laser")
  (Variables|/Game/MainFolder/Scripts/BP_Character.BP_Character_C|SetHasToolBox (Variables|Default|GetAs%20BP%20Character) false)
  (Rendering|SetRenderCustomDepth (Variables|Default|GetStaticMesh) false)
  (Widget|RemovefromParent (Variables|Default|GetHoldWidget)))