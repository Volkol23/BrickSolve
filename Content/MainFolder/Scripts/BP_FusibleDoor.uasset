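; BP_FusibleDoor is a door that opens once when a player carrying a fuse (HasFusible) presses Interact nearby.
; Box overlap checks BP_Character for the fuse, then shows the prompt widget, enables input and opens a Gate, all reversed on exit.
; Interacting passes a DoOnce that tints a dynamic material green, disables collision, calls a 2D sound and plays the skeletal opening animation.
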(event OnComponentBeginOverlap(Box)
  (params (OverlappedComponent :type Primitive%20Component%20Object%20Reference) (OtherActor :type Actor%20Object%20Reference) (OtherComp :type Primitive%20Component%20Object%20Reference) (OtherBodyIndex :type Integer) (bFromSweep :type Boolean) (SweepResult :type Hit%20Result%20Structure%20%28by%20ref%29))
  (bind _asbp_character (Utilities|Casting|CastToBP_Character OtherActor))
  (Variables|Default|SetAs%20BP%20Character _asbp_character)
  (if (Variables|/Game/MainFolder/Scripts/BP_Character.BP_Character_C|GetHasFusible _asbp_character)
    (UserInterface|Viewport|AddtoViewport (Variables|Default|GetInteractW) 0)
    (Input|EnableInput (Game|GetPlayerController 0))
    ;[1 1 1] Widget fusible
    (Utilities|FlowControl|Gate true) ; enters at Open
  ))

(event OnComponentEndOverlap(Box)
  (params (OverlappedComponent :type Primitive%20Component%20Object%20Reference) (OtherActor :type Actor%20Object%20Reference) (OtherComp :type Primitive%20Component%20Object%20Reference) (OtherBodyIndex :type Integer))
  (Utilities|Casting|CastToBP_Character OtherActor)
  (Widget|RemovefromParent (Variables|Default|GetInteractW))
  (Input|DisableInput (Game|GetPlayerController 0))
  ;[1 1 1] Widget fusible
  (Utilities|FlowControl|Gate true) ; enters at Close
)

(event EventBeginPlay
  (bind _returnvalue (UserInterface|CreateWidget "/Game/MainFolder/UI/Interact_Prompt_Widget.Interact_Prompt_Widget_C" (Game|GetPlayerController 0)))
  (Variables|Default|SetInteractW _returnvalue)
  (bind _returnvalue_2 (Rendering|Material|CreateDynamicMaterialInstance "/Game/MainFolder/Assets/Door/Marco_Puerta.Marco_Puerta" "None" "None" :!class /Script/Engine.KismetMaterialLibrary))
  (bind _output_get (Variables|Default|SetPuertaMat _returnvalue_2))
  (Rendering|Material|SetMaterial (Variables|Default|GetdOOR) 0 _output_get))

(event Input|ActionEvents|InputActionInteract
  (params (Key :type Key%20Structure :default "None"))
  (:Pressed
    ;[1 1 1] Widget fusible
    (Utilities|FlowControl|Gate true
      (:Exit
        (Utilities|FlowControl|DoOnce false
          (:Completed
            (Rendering|Material|SetVectorParameterValue (Variables|Default|GetPuertaMat) "Color" "(R=0.232226,G=1.000000,B=0.000000,A=1.000000)" :!class /Script/Engine.MaterialInstanceDynamic)
            (Collision|SetCollisionEnabled (Variables|Default|GetdOOR) "NoCollision")
            ;[1 1 1] Sonido
            (Audio|PlaySound2D 0 1.0 1.0 0.0 0 0)
            (Components|Animation|PlayAnimation (Variables|Default|GetSkeletalMesh) "/Game/MainFolder/Assets/Door/openDoor_Anim.openDoor_Anim" false)))))))

(fn ConstructionScript)