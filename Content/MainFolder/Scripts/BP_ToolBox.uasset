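; BP_ToolBox is a pickup that grants the player character a toolbox and an upgrade mode: Construction, Destruction or Gravity.
; Box overlap by an armed character shows an interact prompt, enables input, outlines the mesh through custom depth and opens a gate for the Interact action.
; Interacting sets the character's mode from UpgradePistolMode and destroys the actor; Destruction and Gravity also replace the character's tutorial text widget.
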(event OnComponentBeginOverlap(Box)
  (params (OverlappedComponent :type Primitive%20Component%20Object%20Reference) (OtherActor :type Actor%20Object%20Reference) (OtherComp :type Primitive%20Component%20Object%20Reference) (OtherBodyIndex :type Integer) (bFromSweep :type Boolean) (SweepResult :type Hit%20Result%20Structure%20%28by%20ref%29))
  (bind _upgradepistolmode (Variables|Default|GetUpgradePistolMode))
  (bind _staticmesh (Variables|Default|GetStaticMesh))
  ;[1 1 1] Enable Interact Options
  (bind _asbp_character (Utilities|Casting|CastToBP_Character OtherActor))
  (bind _output_get (Variables|Default|SetAs%20BP%20Character _asbp_character))
  (if (Variables|/Game/MainFolder/Scripts/BP_Character.BP_Character_C|GetHasWeapon _output_get)
    (UserInterface|Viewport|AddtoViewport (Variables|Default|GetInteractWidget) 0)
    (Input|EnableInput (Game|GetPlayerController 0))
    (Rendering|SetRenderCustomDepth _staticmesh true)
    (Rendering|SetCustomDepthStencilValue _staticmesh 4)
    (Utilities|FlowControl|Gate true) ; enters at Open
  ))

(event OnComponentEndOverlap(Box)
  (params (OverlappedComponent :type Primitive%20Component%20Object%20Reference) (OtherActor :type Actor%20Object%20Reference) (OtherComp :type Primitive%20Component%20Object%20Reference) (OtherBodyIndex :type Integer))
  (bind _upgradepistolmode (Variables|Default|GetUpgradePistolMode))
  (bind _as_bp_character (Variables|Default|GetAs%20BP%20Character))
  ;[1 1 1] Enable Interact Options
  (Utilities|Casting|CastToBP_Character OtherActor)
  (if (Variables|/Game/MainFolder/Scripts/BP_Character.BP_Character_C|GetHasWeapon (stale OnComponentBeginOverlap(Box) _output_get))
    (Widget|RemovefromParent (Variables|Default|GetInteractWidget))
    (Input|DisableInput (Game|GetPlayerController 0))
    (Rendering|SetRenderCustomDepth (Variables|Default|GetStaticMesh) false)
    (Utilities|FlowControl|Gate true) ; enters at Close
  ))

(event EventBeginPlay
  (bind _returnvalue (UserInterface|CreateWidget "/Game/MainFolder/UI/Interact_Prompt_Widget.Interact_Prompt_Widget_C" (Game|GetPlayerController 0)))
  (Variables|Default|SetInteractWidget _returnvalue))

(event Input|ActionEvents|InputActionInteract
  (params (Key :type Key%20Structure :default "None"))
  (bind _upgradepistolmode (Variables|Default|GetUpgradePistolMode))
  (bind _as_bp_character (Variables|Default|GetAs%20BP%20Character))
  ;[1 1 1] Enable Interact Options
  (:Pressed
    (Utilities|FlowControl|Gate true
      (:Exit
        (Variables|/Game/MainFolder/Scripts/BP_Character.BP_Character_C|SetHasToolBox (Variables|Default|GetAs%20BP%20Character) true)
        (Development|PrintString (Utilities|String|EnumtoString _upgradepistolmode))
        (switch Utilities|FlowControl|Switch|SwitchonPistolMode _upgradepistolmode
          (:NewEnumerator1
            (Variables|/Game/MainFolder/Scripts/BP_Character.BP_Character_C|SetUpgradeMode _as_bp_character "NewEnumerator0")
            (Utilities|FlowControl|Sequence
              (:then_0
                (Actor|DestroyActor))))
          (:NewEnumerator2
            (Variables|/Game/MainFolder/Scripts/BP_Character.BP_Character_C|SetUpgradeMode _as_bp_character "NewEnumerator1")
            (Actor|DestroyActor :!label _label)
            (Default|RemoveTextWidget (Variables|Default|GetAs%20BP%20Character))
            (bind _returnvalue (UserInterface|CreateWidget "/Game/UI/TextBeforePickUP/TutorialWidget1.TutorialWidget1_C" (Game|GetPlayerController 0)))
            (Variables|/Game/MainFolder/Scripts/BP_Character.BP_Character_C|SetWidgetText (Variables|Default|GetAs%20BP%20Character) _returnvalue)
            (bind _output_get (Variables|Default|SetTutorialWidgets _returnvalue))
            (Variables|/Game/UI/TextBeforePickUP/TutorialWidget1.TutorialWidget1_C|SetInputText _output_get (Variables|Default|GetInput%20Text))
            (UserInterface|Viewport|AddtoViewport (Variables|Default|GetTutorialWidgets) 0))
          (:NewEnumerator3
            (Variables|/Game/MainFolder/Scripts/BP_Character.BP_Character_C|SetUpgradeMode _as_bp_character "NewEnumerator2")
            (goto _label)))))))

(fn ConstructionScript)