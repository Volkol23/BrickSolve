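; BP_GravityCounter tracks whether all gravity objects sit in their target positions, apparently for a placement puzzle.
; Until complete, Tick loops over GravityObjects, reading ObjectOnPosition to adjust a clamped Counter.
; Shared DoOnce nodes, reset after each incomplete check, limit changes to one increment and one decrement per pass, so Counter is not a true tally.
; When Counter equals the array length, TotalObjectsPlaced latches and Tick only prints a placeholder string.
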(event Custom|CheckPlacedObjects
  (bind _gravityobjects (Variables|Default|GetGravityObjects))
  ;[1 1 1] Check number Of Objects Placed in their positions
  (for _array_element _gravityobjects
    (if (Variables|/Game/MainFolder/Scripts/BP_GravityObject.BP_GravityObject_C|GetObjectOnPosition _array_element)
      (Utilities|FlowControl|DoOnce false
        (:Completed
          (bind _result (Math|Integer|IncrementInt (Variables|Default|GetCounter))
            (:%20%20
              (Variables|Default|SetCounter (Math|Integer|Clamp(Integer) _result 0 4))))))
      (else
        (Utilities|FlowControl|DoOnce false
          (:Completed
            (bind _result_2 (Math|Integer|DecrementInt (Variables|Default|GetCounter))
              (:%20%20
                (Variables|Default|SetCounter (Math|Integer|Clamp(Integer) _result_2 0 4)))))))))
  (if (== (Variables|Default|GetCounter) (Utilities|Array|Length _gravityobjects))
    (Variables|Default|SetTotalObjectsPlaced true)
    (else
      (Utilities|FlowControl|Sequence
        (:then_0
          (Utilities|FlowControl|DoOnce false) ; enters at Reset
        )
        (:then_1
          (Utilities|FlowControl|DoOnce false) ; enters at Reset
        )))))

(event EventTick
  (params (DeltaSeconds :type Float%20%28single-precision%29))
  (if (Variables|Default|GetTotalObjectsPlaced)
    (Development|PrintString "DoSomething")
    (else
      (CallFunction|CheckPlacedObjects))))

(fn ConstructionScript)