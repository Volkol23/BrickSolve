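; Pickup actor that the player collects by pressing E inside its Box, showing a text message before it disappears.
; Box overlaps with the fesfses class show or hide the interact prompt, toggle input and open or close a gate on the key.
; Pressing E destroys mesh and box, displays the InteractionText widget, waits TimeToFinish, triggers its fade and destroys the actor.
; Both widgets are created at BeginPlay.
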(event OnComponentEndOverlap(Box)
  (params (OverlappedComponent :type Primitive%20Component%20Object%20Reference) (OtherActor :type Actor%20Object%20Reference) (OtherComp :type Primitive%20Component%20Object%20Reference) (OtherBodyIndex :type Integer))
  (bind _interactionpromptref (Variables|Default|GetInteractionPromptREF))
  (Utilities|Casting|CastTofesfses OtherActor)
  (Widget|RemovefromParent (Variables|Default|GetInteractPrompt%20REF))
  (Input|DisableInput (Game|GetPlayerController 0))
  (Utilities|FlowControl|Gate true) ; enters at Close
)

(event OnComponentBeginOverlap(Box)
  (params (OverlappedComponent :type Primitive%20Component%20Object%20Reference) (OtherActor :type Actor%20Object%20Reference) (OtherComp :type Primitive%20Component%20Object%20Reference) (OtherBodyIndex :type Integer) (bFromSweep :type Boolean) (SweepResult :type Hit%20Result%20Structure%20%28by%20ref%29))
  (bind _interactionpromptref (Variables|Default|GetInteractionPromptREF))
  (Utilities|Casting|CastTofesfses OtherActor)
  (UserInterface|Viewport|AddtoViewport (Variables|Default|GetInteractPrompt%20REF) 0)
  (Input|EnableInput (Game|GetPlayerController 0))
  (Variables|/Game/UI/TextBeforePickUP/InteractionPrompt_Widget.InteractionPrompt_Widget_C|SetInteractionText _interactionpromptref (Variables|Default|GetInteraction%20Text))
  (Utilities|FlowControl|Gate true) ; enters at Open
)

(event EventBeginPlay
  (Utilities|FlowControl|Sequence
    (:then_0
      (bind _returnvalue (UserInterface|CreateWidget "/Game/UI/InteractText/Interact_Prompt_Widget.Interact_Prompt_Widget_C"))
      (Variables|Default|SetInteractPrompt%20REF _returnvalue))
    (:then_1
      (bind _returnvalue_2 (UserInterface|CreateWidget "/Game/UI/TextBeforePickUP/InteractionPrompt_Widget.InteractionPrompt_Widget_C"))
      (Variables|Default|SetInteractionPromptREF _returnvalue_2))))

(event Input|KeyboardEvents|E
  (params (Key :type Key%20Structure :default "None"))
  (bind _interactionpromptref (Variables|Default|GetInteractionPromptREF))
  (:Pressed
    (Utilities|FlowControl|Gate true
      (:Exit
        (Components|DestroyComponent (Variables|Default|GetStaticMesh))
        (UserInterface|Viewport|AddtoViewport _interactionpromptref 0)
        (Utilities|FlowControl|Delay (Variables|Default|GetTimeToFinish))
        (Default|FadeEnd _interactionpromptref)
        (Actor|DestroyActor)))))

(fn ConstructionScript)