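; BP_AutomaticDoor is a two-panel sliding door that opens when a BP_Character overlaps its Trigger while IsOpen is false.
; OpenDoor and CloseDoor use separate timelines per panel to lerp relative Y from its current value toward fixed targets.
; Collision is disabled on opening and restored to query-only after the left panel closes.
; IsOpen updates when the right panel finishes; CloseDoor has no caller in this graph.
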(event OnComponentBeginOverlap(Trigger)
  (params (OverlappedComponent :type Primitive%20Component%20Object%20Reference) (OtherActor :type Actor%20Object%20Reference) (OtherComp :type Primitive%20Component%20Object%20Reference) (OtherBodyIndex :type Integer) (bFromSweep :type Boolean) (SweepResult :type Hit%20Result%20Structure%20%28by%20ref%29))
  (Utilities|Casting|CastToBP_Character OtherActor)
  (if (not (Variables|Default|GetIsOpen))
    (CallFunction|OpenDoor)))

(event Custom|OpenDoor
  (bind _doorright (Variables|Default|GetDoorRight))
  ;[1 1 1] Open Automatic Door
  (Utilities|FlowControl|Sequence
    (:then_0
      (Collision|SetCollisionEnabled (Variables|Default|GetLeftDoor) "NoCollision")
      (bind _alphalocation (Timeline|Timeline_0 PlayFromStart)
        (:Update
          (Transformation|SetRelativeLocation (Variables|Default|GetLeftDoor) (Math|Vector|MakeVector 0.0 (Math|Float|Lerp (.y (Variables|/Script/Engine.SceneComponent|GetRelativeLocation (Variables|Default|GetLeftDoor))) 7.0 _alphalocation) 0.0) false false))))
    (:then_1
      (bind _alphalocation_2 (Timeline|Timeline_1 PlayFromStart)
        (:Update
          (Transformation|SetRelativeLocation _doorright (Math|Vector|MakeVector 0.0 (Math|Float|Lerp (.y (Variables|/Script/Engine.SceneComponent|GetRelativeLocation (Variables|Default|GetDoorRight))) -8.0 _alphalocation_2) 0.0) false false))
        (:Finished
          (Collision|SetCollisionEnabled _doorright "NoCollision")
          (Variables|Default|SetIsOpen true))))))

(event Custom|CloseDoor
  (bind _doorright (Variables|Default|GetDoorRight))
  ;[1 1 1] Close Automatic Door
  (Utilities|FlowControl|Sequence
    (:then_0
      (bind _alphalocation (Timeline|Timeline_2 PlayFromStart)
        (:Update
          (Transformation|SetRelativeLocation (Variables|Default|GetLeftDoor) (Math|Vector|MakeVector 0.0 (Math|Float|Lerp (.y (Variables|/Script/Engine.SceneComponent|GetRelativeLocation (Variables|Default|GetLeftDoor))) 0.0 _alphalocation) 0.0) false false))
        (:Finished
          (Collision|SetCollisionEnabled (Variables|Default|GetLeftDoor) "QueryOnly"))))
    (:then_1
      (Collision|SetCollisionEnabled _doorright "NoCollision")
      (bind _alphalocation_2 (Timeline|Timeline_3 PlayFromStart)
        (:Update
          (Transformation|SetRelativeLocation _doorright (Math|Vector|MakeVector 0.0 (Math|Float|Lerp (.y (Variables|/Script/Engine.SceneComponent|GetRelativeLocation (Variables|Default|GetDoorRight))) 0.0 _alphalocation_2) 0.0) false false))
        (:Finished
          (Variables|Default|SetIsOpen false))))))

(fn ConstructionScript)