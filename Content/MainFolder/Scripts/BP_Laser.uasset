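; Laser beam actor for the player's pistol, acting on what it hits according to the character's current pistol mode.
; Each Tick it line-traces forward while the player fires, updates the Niagara beam and hit effect positions, and colors the effects by mode.
; Construction and Gravity send messages to the hit actor, while Destruction applies radius damage to destructible objects.
; StopLaser deactivates the effects, plays a scale timeline, then destroys the actor.
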(event Custom|Stop%20Laser
  ;[1 1 1] Stop Laser
  (Utilities|FlowControl|DoOnce false
    (:Completed
      (Components|Activation|Deactivate (Variables|Default|GetLaser))
      (Components|Activation|Deactivate (Variables|Default|GetWeapon_Fire))
      (Components|Activation|Deactivate (Variables|Default|GetLaser_Hit))
      (bind _scale (Timeline|LaserDeactivate PlayFromStart)
        (:Update
          (Effects|Components|ParticleSystem|SetFloatParameter (Variables|Default|GetLaser) "User.Scale" _scale))
        (:Finished
          (Actor|DestroyActor))))))

(event EventTick
  (params (DeltaSeconds :type Float%20%28single-precision%29))
  (bind _returnvalue (Game|GetPlayerCharacter 0))
  (bind _asbp_character (Utilities|Casting|CastToBP_Character _returnvalue))
  (bind _pistolmode (Variables|/Game/MainFolder/Scripts/BP_Character.BP_Character_C|GetPistolMode _asbp_character))
  ;[1 1 1] Laser Behaviour
  (bind _outhit (CallFunction|EmitLaser))
  (Variables|Default|SetHitActor (.HitActor (Collision|BreakHitResult _outhit)))
  (Variables|Default|SetImpact%20Normal (.ImpactNormal (Collision|BreakHitResult _outhit)))
  (Variables|Default|SetLocation (.Location (Collision|BreakHitResult _outhit)))
  (Effects|Components|ParticleSystem|SetVectorParameter (Variables|Default|GetLaser) "User.BeamEnd" (Math|Vector|SelectVector (.Location (Collision|BreakHitResult _outhit)) (.TraceEnd (Collision|BreakHitResult _outhit)) (Utilities|IsValid (.HitActor (Collision|BreakHitResult _outhit)))))
  (Variables|Default|SetPistol%20Mode _pistolmode)
  (CallFunction|SetLaserMode _pistolmode)
  (Effects|Components|ParticleSystem|SetVectorParameter (Variables|Default|GetLaser_Hit) "User.HitLocation" (Variables|Default|GetLocation))
  (switch Utilities|FlowControl|Switch|SwitchonPistolMode (Variables|Default|GetPistol%20Mode)
    (:NewEnumerator1
      (Class|IConstruction|Construct(Message) (Variables|Default|GetHitActor) (Variables|Default|GetPistol%20Mode)))
    (:NewEnumerator2
      ;[1 1 1] Destruction Effect
      (bind _asbp_destructible_object (Utilities|Casting|CastToBP_DestructibleObject (Variables|Default|GetHitActor)))
      (if (not (Variables|/Game/MainFolder/Scripts/BP_DestructibleObject.BP_DestructibleObject_C|GetisDestroyed _asbp_destructible_object))
        (if (> (.x (Variables|Default|GetImpact%20Normal)) 0.0)
          (Class|DestructibleComponent|ApplyRadiusDamage (Variables|/Script/ApexDestruction.DestructibleActor|GetDestructibleComponent _asbp_destructible_object) 2.0 (Variables|Default|GetLocation) 0.0 2e+02 true)
          (Class|IDestruction|Destruct(Message) (Variables|Default|GetHitActor) (Variables|Default|GetPistol%20Mode)))))
    (:NewEnumerator3
      (Class|IGravity|GravityEffect(Message) (Variables|Default|GetHitActor) (Variables|Default|GetPistol%20Mode)))))

(fn ConstructionScript)

(fn EmitLaser
  (bind _scene (Variables|Default|GetScene))
  (bind _returnvalue (Transformation|GetWorldLocation _scene))
  (if (Variables|/Game/MainFolder/Scripts/BP_Character.BP_Character_C|GetisFiring (.AsBP%20Character (Utilities|Casting|CastToBP_Character (Game|GetPlayerCharacter 0))))
    (bind _outhit (Collision|LineTraceByChannel _returnvalue (+ _returnvalue (* (Math|Vector|GetForwardVector _scene) (Variables|Default|GetWeaponRange))) "TraceTypeQuery1" false 0 "None" true "(R=1.000000,G=0.000000,B=0.000000,A=1.000000)" "(R=0.000000,G=1.000000,B=0.000000,A=1.000000)" 0.0))
    (return _outhit)))

(fn SetLaserMode
  (params (PistolMode :type PistolMode%20Enum :default "NewEnumerator0"))
  (switch Utilities|FlowControl|Switch|SwitchonPistolMode PistolMode
    (:NewEnumerator0
      (CallFunction|SetColor (Variables|Default|GetWhite)))
    (:NewEnumerator1
      (CallFunction|SetColor (Variables|Default|GetBlue)))
    (:NewEnumerator2
      (CallFunction|SetColor (Variables|Default|GetRed)))
    (:NewEnumerator3
      (CallFunction|SetColor (Variables|Default|GetGreen)))))

(fn SetColor
  (params (Color :type Linear%20Color%20Structure))
  (Effects|Components|ParticleSystem|SetColorParameter (Variables|Default|GetLaser) "Color" Color)
  (Effects|Components|ParticleSystem|SetColorParameter (Variables|Default|GetLaser_Hit) "Color" Color)
  (Effects|Components|ParticleSystem|SetColorParameter (Variables|Default|GetWeapon_Fire) "Color" Color))