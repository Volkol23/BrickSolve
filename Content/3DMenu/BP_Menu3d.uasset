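; 3D menu actor that hosts a widget and moves the player's view between linked menu actors.
; On begin play it binds to the Menu3dWidget transition event and disables its own collision.
; The widget's index picks a target from LinkedMenus, then the view target blends to that actor with ease in-out.
; Collision switches from the current menu to the new one during each transition.
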(event Custom|TransitionTo
  (params (NewMenu :type BP%20Menu%203d%20Object%20Reference))
  (Collision|SetActorEnableCollision false)
  (Collision|SetActorEnableCollision NewMenu true)
  (Game|Player|SetViewTargetwithBlend (Game|GetPlayerController 0) NewMenu 2.0 "VTBlend_EaseInOut" 2.0 false))

(event Custom|OnTransitionBetweenMenus
  (params (MenuIndex :type Integer))
  (if (Utilities|Array|IsValidIndex (Variables|Default|GetLinkedMenus) MenuIndex)
    (CallFunction|Transitionto (Utilities|Array|Get(acopy) (Variables|Default|GetLinkedMenus) MenuIndex))))

(event EventBeginPlay
  (Utilities|FlowControl|Sequence
    (:then_0
      (bind _asmenu_3d_widget (Utilities|Casting|CastToMenu3dWidget (UserInterface|GetUserWidgetObject (Variables|Default|GetWidget))))
      (EventDispatchers|BindEventtoTransitiontoLinkedMenu _asmenu_3d_widget (delegate Custom|OnTransitionBetweenMenus))
      (Collision|SetActorEnableCollision false))))

(fn ConstructionScript)