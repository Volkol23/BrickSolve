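; BP_Checkpoint is a placeable checkpoint that updates the player's respawn point.
; When a BP_Character overlaps its Box trigger, it passes the world location of its SpawnLoc component to the character's NewSpawnLocation function.
; The construction script sizes the box and positions SpawnLoc from the InBoxExtent and SpawnPointVector variables, so both can be set per instance.
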(event OnComponentBeginOverlap(Box)
  (params (OverlappedComponent :type Primitive%20Component%20Object%20Reference) (OtherActor :type Actor%20Object%20Reference) (OtherComp :type Primitive%20Component%20Object%20Reference) (OtherBodyIndex :type Integer) (bFromSweep :type Boolean) (SweepResult :type Hit%20Result%20Structure%20%28by%20ref%29))
  (bind _asbp_character (Utilities|Casting|CastToBP_Character OtherActor))
  (Default|NewSpawnLocation _asbp_character (Transformation|GetWorldLocation (Variables|Default|GetSpawnLoc))))

(event EventBeginPlay
  (Utilities|Casting|CastToBP_Character (Game|GetPlayerCharacter 0)))

(fn ConstructionScript
  (Components|Box|SetBoxExtent (Variables|Default|GetBox) (Variables|Default|GetIn%20Box%20Extent) true)
  (Transformation|SetRelativeLocation (Variables|Default|GetSpawnLoc) (Variables|Default|GetSpawnPoint%20Vector) false false))