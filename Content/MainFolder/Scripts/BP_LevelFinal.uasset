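; BP_LevelFinal is a level-end trigger that shows the FinalLevel screen when the player character reaches it.
; A Box overlap casts the other actor to BP_Character, disables its input, then adds the FinalLevel widget to the viewport.
; It then pauses the game, shows the mouse cursor and switches to UI-only input with the mouse locked in fullscreen.
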(event OnComponentBeginOverlap(Box)
  (params (OverlappedComponent :type Primitive%20Component%20Object%20Reference) (OtherActor :type Actor%20Object%20Reference) (OtherComp :type Primitive%20Component%20Object%20Reference) (OtherBodyIndex :type Integer) (bFromSweep :type Boolean) (SweepResult :type Hit%20Result%20Structure%20%28by%20ref%29))
  (bind _returnvalue (Game|GetPlayerController 0))
  (Development|PrintString "Enter Final")
  (bind _asbp_character (Utilities|Casting|CastToBP_Character OtherActor))
  (if true
    (Input|DisableInput _asbp_character (Game|GetPlayerController 0))
    (bind _returnvalue_2 (UserInterface|CreateWidget "/Game/MainFolder/UI/FinalLevel.FinalLevel_C" (Game|GetPlayerController 0)))
    (UserInterface|Viewport|AddtoViewport _returnvalue_2 0)
    (Development|PrintString "Widget created")
    (Game|SetGamePaused true)
    (Variables|/Script/Engine.PlayerController|SetbShowMouseCursor _returnvalue true)
    (Input|SetInputModeUIOnly _returnvalue 0 "LockInFullscreen")))

(event EventBeginPlay)

(event Collision|EventActorBeginOverlap
  (params (OtherActor :type Actor%20Object%20Reference)))

(event EventTick
  (params (DeltaSeconds :type Float%20%28single-precision%29)))

(fn ConstructionScript)