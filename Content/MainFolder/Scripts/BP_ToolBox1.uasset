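; BP_ToolBox1 is an interactable toolbox that clears the player character's HasFusible flag and destroys itself when used.
; It creates an interact prompt widget at BeginPlay.
; Box overlap with BP_Character shows the prompt, enables input and outlines the mesh through custom depth stencil, reversing these on exit.
; A gate, open only during overlap, lets the Interact press through.
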(event OnComponentBeginOverlap(Box)
  (params (OverlappedComponent :type Primitive%20Component%20Object%20Reference) (OtherActor :type Actor%20Object%20Reference) (OtherComp :type Primitive%20Component%20Object%20Reference) (OtherBodyIndex :type Integer) (bFromSweep :type Boolean) (SweepResult :type Hit%20Result%20Structure%20%28by%20ref%29))
  (bind _staticmesh (Variables|Default|GetStaticMesh))
  ;[1 1 1] Enable Interact Options
  (bind _asbp_character (Utilities|Casting|CastToBP_Character OtherActor))
  (Variables|Default|SetAs%20BP%20Character _asbp_character)
  (UserInterface|Viewport|AddtoViewport (Variables|Default|GetInteractWidget) 0)
  (Input|EnableInput (Game|GetPlayerController 0))
  (Rendering|SetRenderCustomDepth _staticmesh true)
  (Rendering|SetCustomDepthStencilValue _staticmesh 4)
  (Utilities|FlowControl|Gate true) ; enters at Open
)

(event OnComponentEndOverlap(Box)
  (params (OverlappedComponent :type Primitive%20Component%20Object%20Reference) (OtherActor :type Actor%20Object%20Reference) (OtherComp :type Primitive%20Component%20Object%20Reference) (OtherBodyIndex :type Integer))
  ;[1 1 1] Enable Interact Options
  (Utilities|Casting|CastToBP_Character OtherActor)
  (Widget|RemovefromParent (Variables|Default|GetInteractWidget))
  (Input|DisableInput (Game|GetPlayerController 0))
  (Rendering|SetRenderCustomDepth (Variables|Default|GetStaticMesh) false)
  (Utilities|FlowControl|Gate true) ; enters at Close
)

(event EventBeginPlay
  (bind _returnvalue (UserInterface|CreateWidget "/Game/MainFolder/UI/Interact_Prompt_Widget.Interact_Prompt_Widget_C" (Game|GetPlayerController 0)))
  (Variables|Default|SetInteractWidget _returnvalue))

(event Input|ActionEvents|InputActionInteract
  (params (Key :type Key%20Structure :default "None"))
  ;[1 1 1] Enable Interact Options
  (:Pressed
    (Utilities|FlowControl|Gate true
      (:Exit
        (Variables|/Game/MainFolder/Scripts/BP_Character.BP_Character_C|SetHasFusible (Variables|Default|GetAs%20BP%20Character) false)
        (Actor|DestroyActor)))))

(fn ConstructionScript)