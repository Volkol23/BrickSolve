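; BP_Fusible is a pickup actor that gives BP_Character a fusible, likely a fuse, when the player interacts nearby.
; It creates an interact prompt widget on BeginPlay, and box overlap with the character shows or hides it while toggling input and a Gate.
; Interact passes through the open Gate, sets HasFusible on the character and destroys the actor.
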(event OnComponentBeginOverlap(Box)
  (params (OverlappedComponent :type Primitive%20Component%20Object%20Reference) (OtherActor :type Actor%20Object%20Reference) (OtherComp :type Primitive%20Component%20Object%20Reference) (OtherBodyIndex :type Integer) (bFromSweep :type Boolean) (SweepResult :type Hit%20Result%20Structure%20%28by%20ref%29))
  (bind _asbp_character (Utilities|Casting|CastToBP_Character OtherActor))
  (Variables|Default|SetAs%20BP%20Character _asbp_character)
  (UserInterface|Viewport|AddtoViewport (Variables|Default|GetINTERACT%20wIDGET) 0)
  (Input|EnableInput 0)
  (Utilities|FlowControl|Gate true) ; enters at Open
)

(event OnComponentEndOverlap(Box)
  (params (OverlappedComponent :type Primitive%20Component%20Object%20Reference) (OtherActor :type Actor%20Object%20Reference) (OtherComp :type Primitive%20Component%20Object%20Reference) (OtherBodyIndex :type Integer))
  (Utilities|Casting|CastToBP_Character OtherActor)
  (Widget|RemovefromParent (Variables|Default|GetINTERACT%20wIDGET))
  (Input|DisableInput 0)
  (Utilities|FlowControl|Gate true) ; enters at Close
)

(event EventBeginPlay
  (bind _returnvalue (UserInterface|CreateWidget "/Game/MainFolder/UI/Interact_Prompt_Widget.Interact_Prompt_Widget_C"))
  (Variables|Default|SetINTERACT%20wIDGET _returnvalue))

(event Input|ActionEvents|InputActionInteract
  (params (Key :type Key%20Structure :default "None"))
  (:Pressed
    (Utilities|FlowControl|Gate true
      (:Exit
        (Variables|/Game/MainFolder/Scripts/BP_Character.BP_Character_C|SetHasFusible (Variables|Default|GetAs%20BP%20Character) true)
        (Actor|DestroyActor)))))

(fn ConstructionScript)