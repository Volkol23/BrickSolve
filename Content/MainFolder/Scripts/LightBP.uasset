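; LightBP is a numbered spotlight actor with a god ray mesh that is switched on through a LightON event.
; The construction script applies per-instance mesh, intensity, attenuation radius and cone angle, and writes the light's number to a text render.
; BeginPlay creates a dynamic god ray material.
; LightON shows light and ray, disables the ray's collision responses, and plays a timeline driving the material's Transparency.
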(event Custom|LightON
  (bind _godray (Variables|Default|GetGodRay))
  (Collision|SetCollisionResponsetoAllChannels _godray "ECR_Ignore")
  (Rendering|SetVisibility (Variables|Default|GetSpotLight) true false)
  (Rendering|Material|SetMaterial _godray 0 (Variables|Default|GetGodRayMAT))
  (Rendering|SetVisibility _godray true false)
  (bind _newtrack_0 (Timeline|Timeline_0 Play)
    (:Update
      (Rendering|Material|SetScalarParameterValue (Variables|Default|GetGodRayMAT) "Transparency" _newtrack_0 :!class /Script/Engine.MaterialInstanceDynamic))))

(event EventBeginPlay
  (bind _returnvalue (Rendering|Material|CreateDynamicMaterialInstance "/Game/MainFolder/Particles/GodRayMat_Inst.GodRayMat_Inst" "None" "None" :!class /Script/Engine.KismetMaterialLibrary))
  (Variables|Default|SetGodRayMAT _returnvalue))

(event Collision|EventActorBeginOverlap
  (params (OtherActor :type Actor%20Object%20Reference)))

(event EventTick
  (params (DeltaSeconds :type Float%20%28single-precision%29)))

(fn ConstructionScript
  (bind _spotlight (Variables|Default|GetSpotLight))
  (Components|StaticMesh|SetStaticMesh (Variables|Default|GetGodRay) (Variables|Default|GetGodRayMesh))
  (Rendering|Components|Light|SetIntensity _spotlight (Variables|Default|GetNew%20Intensity))
  (Rendering|Lighting|SetAttenuationRadius _spotlight (Variables|Default|GetAttenueationRadius))
  (Rendering|Lighting|SetOuterConeAngle _spotlight (Variables|Default|GetNew%20Outer%20Cone%20Angle))
  (Rendering|Components|TextRender|SetText (Variables|Default|GetTextRender) (Utilities|Text|ToText(Integer) (Variables|Default|GetNumber)))
  (Rendering|SetBoundsScale (Variables|Default|GetTextRender) 22.0))