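; BP_GravityObject is a gravity holder that captures its ObjectToMove when that component enters trigger W.
; Grab teleports it to the Arrow, attaches it to a physics constraint and ignores Pawn collision.
; In launch pad mode it only grabs; otherwise it flags the object in position and steps Niagara colors through delays before Drop.
; Drop breaks the constraint, restores Pawn blocking and launches the object with a fixed impulse.
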(event OnComponentBeginOverlap(w)
  (params (OverlappedComponent :type Primitive%20Component%20Object%20Reference) (OtherActor :type Actor%20Object%20Reference) (OtherComp :type Primitive%20Component%20Object%20Reference) (OtherBodyIndex :type Integer) (bFromSweep :type Boolean) (SweepResult :type Hit%20Result%20Structure%20%28by%20ref%29))
  (bind _niagara (Variables|Default|GetNiagara))
  (if (== OtherComp (Variables|Default|GetObjectToMove))
    (if (Variables|Default|GetIsLaunchPad)
      (CallFunction|Grab)
      (else
        (CallFunction|Grab)
        (Variables|Default|SetObjectOnPosition true)
        (Utilities|FlowControl|Delay 1.0)
        (Effects|Components|ParticleSystem|SetColorParameter _niagara "Color" "(R=1.999998,G=1.236483,B=0.593749,A=1.000000)")
        (Utilities|FlowControl|Delay 2.0)
        (Effects|Components|ParticleSystem|SetColorParameter _niagara "Color" "(R=10.000000,G=0.000000,B=0.394378,A=1.000000)")
        (Utilities|FlowControl|Delay 3.0)
        (CallFunction|Drop)))))

(event OnComponentEndOverlap(w)
  (params (OverlappedComponent :type Primitive%20Component%20Object%20Reference) (OtherActor :type Actor%20Object%20Reference) (OtherComp :type Primitive%20Component%20Object%20Reference) (OtherBodyIndex :type Integer))
  (if (== OtherComp (Variables|Default|GetObjectToMove))
    (Effects|Components|ParticleSystem|SetColorParameter (Variables|Default|GetNiagara) "Color" "(R=0.000000,G=10.000000,B=2.000000,A=1.000000)")))

(event EventBeginPlay
  (bind _asbp_character (Utilities|Casting|CastToBP_Character (Game|GetPlayerCharacter 0)))
  (Variables|Default|SetAs%20BP%20Character _asbp_character))

(fn ConstructionScript)

(fn Grab
  (bind _objecttomove (Variables|Default|GetObjectToMove))
  (Transformation|SetWorldLocation _objecttomove (Transformation|GetWorldLocation (Variables|Default|GetArrow)) false true)
  (Class|PhysicsConstraintComponent|SetConstrainedComponents (Variables|Default|GetPhysicsConstraint) _objecttomove "None" 0 "None")
  (Collision|SetCollisionResponsetoChannel _objecttomove "ECC_Pawn" "ECR_Ignore"))

(fn Drop
  (bind _objecttomove (Variables|Default|GetObjectToMove))
  (Class|PhysicsConstraintComponent|BreakConstraint (Variables|Default|GetPhysicsConstraint))
  (Utilities|IsValid _objecttomove
    (:Is%20Valid
      (Collision|SetCollisionResponsetoChannel _objecttomove "ECC_Pawn" "ECR_Block")
      (Physics|AddImpulse _objecttomove "5000.000000,10000.000000,50000.000000" "None" false)
      (Variables|Default|SetObjectOnPosition false))))